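; Player controller for a prop hunt game that creates the main HUD widget for the local player and relays game state to it.
; BeginPlay builds W_MainHUD on clients and on a locally controlled authority.
; Wrapper events forward prop role, health, countdown, win screen and crosshair hit feedback to matching "OnClient" events that update the HUD.
; The stored prop role is passed along with the match result to the win screen.
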(event Custom|SetPropOnClient
  (params (isProp? :type Boolean))
  (Default|SetUpPropWidget (Variables|Default|GetMainHudGraf) isProp?))

(event Custom|UpdateHealtOnClient
  (params (Healt :type Float%20%28double-precision%29))
  (Default|UpdateHealtBar (Variables|Default|GetMainHudGraf) Healt))

(event Custom|ShowWinScreenOnClient
  (params (PropWon? :type Boolean) (IsProp? :type Boolean))
  (Default|ShowWinScreen (Variables|Default|GetMainHudGraf) PropWon? IsProp?))

(event Custom|StartCountDownOnClient
  (Default|StartTimer (Variables|Default|GetMainHudGraf)))

(event Custom|ShowCrosshairHitOnClient
  (Default|PlayHitAnimation (Variables|Default|GetMainHudGraf)))

(event EventUpdateHealthWidget
  (params (Healt :type Float%20%28double-precision%29))
  (CallFunction|UpdateHealtonClient Healt))

(event EventShowWinScreenWidget
  (params (PropWon? :type Boolean))
  (CallFunction|ShowWinScreenonClient PropWon? (Variables|Default|GetIs%20Prop?)))

(event EventBeginPlay
  ;[1 1 1] Create Widget For Client
  (Networking|SwitchHasAuthority
    (:Authority
      (if (Pawn|IsLocalPlayerController)
        (bind _returnvalue (UserInterface|CreateWidget "/Game/Core/Widgets/W_MainHUD.W_MainHUD_C" self :!label _label))
        (bind _output_get (Variables|Default|SetMainHudGraf _returnvalue))
        (UserInterface|Viewport|AddtoViewport _output_get 0)))
    (:Remote
      (goto _label))))

(event EventStartCountDownWidget
  (CallFunction|StartCountDownonClient))

(event EventSetUpPorpWidget
  (params (isProp? :type Boolean))
  (Variables|Default|SetIs%20Prop? isProp?)
  (CallFunction|SetProponClient isProp?))

(event EventPlayCrosshairHit
  (CallFunction|ShowCrosshairHitonClient))

(fn ConstructionScript)